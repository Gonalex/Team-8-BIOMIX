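; JumpPadBP is an environmental jump pad that launches the player character when it overlaps the pad.
; On overlap it applies a Velocity launch with Z override, then calls Launch to animate the pad.
; Launch plays a timeline that lerps the Cylinder and Cube support upward from their current positions by a fixed offset.
; A CanLaunch flag blocks retriggering until the timeline finishes.
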(event Custom|Launch
  (Variables|Default|SetCurrent%20Jump%20Pad%20Location (Transformation|GetWorldLocation (Variables|Default|GetCylinder)))
  (Variables|Default|SetCurrent%20Support%20Location (Transformation|GetWorldLocation (Variables|Default|GetCube)))
  (bind _newtrack_0 (Timeline|Timeline_0 PlayFromStart)
    (:Update
      (Utilities|FlowControl|Sequence
        (:then_0
          (Transformation|SetWorldLocation (Variables|Default|GetCylinder) (Math|Vector|Lerp(Vector) (Variables|Default|GetCurrent%20Jump%20Pad%20Location) (+ (Variables|Default|GetCurrent%20Jump%20Pad%20Location) "0, 0,80.000000") _newtrack_0) false false))
        (:then_1
          (Transformation|SetWorldLocation (Variables|Default|GetCube) (Math|Vector|Lerp(Vector) (Variables|Default|GetCurrent%20Support%20Location) (+ (Variables|Default|GetCurrent%20Support%20Location) "0, 0,80.000000") _newtrack_0) false false))))
    (:Finished
      (Variables|Default|SetCan%20Launch true))))

(event Collision|EventActorBeginOverlap
  (params (OtherActor :type Actor%20Object%20Reference))
  (bind _returnvalue (Game|Player|GetPlayerPawn 0))
  ;[0 0 1] Jump Pad
  (if (== OtherActor _returnvalue)
    (if (Variables|Default|GetCan%20Launch)
      (Variables|Default|SetCan%20Launch false)
      (bind _ascharacter (Utilities|Casting|CastToCharacter _returnvalue))
      (Character|LaunchCharacter _ascharacter (Variables|Default|GetVelocity) false true)
      (CallFunction|Launch))))

(fn ConstructionScript)