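; Spike trap Blueprint, apparently a test, that extends and retracts a Cone component and damages the player on contact.
; The inherited ActivateTrap event plays a Move timeline that lerps the cone out, then reverses it after a delay; DoOnce gates with no reset limit this to one cycle.
; Cone overlap with SideScrollerCharacter starts a self-calling Redamage loop that applies timed damage until end overlap clears the stored actor.
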(event OnComponentBeginOverlap(Cone)
  (params (OverlappedComponent :type Primitive%20Component%20Object%20Reference) (OtherActor :type Actor%20Object%20Reference) (OtherComp :type Primitive%20Component%20Object%20Reference) (OtherBodyIndex :type Integer) (bFromSweep :type Boolean) (SweepResult :type Hit%20Result%20Structure%20%28by%20ref%29))
  ;[1 0 0.7416] Applies damage to player when overlapping.
  (Variables|Default|SetOverlappedActor OtherActor)
  (if (== (Utilities|GetClass OtherActor) "/Game/SynthvaniaContent/Blueprints/SideScrollerCharacter.SideScrollerCharacter_C")
    (Game|Damage|ApplyDamage (Variables|Default|GetOverlappedActor) 5.0 0 0)
    (Utilities|FlowControl|Delay 0.5)
    (CallFunction|Redamage)))

(event OnComponentEndOverlap(Cone)
  (params (OverlappedComponent :type Primitive%20Component%20Object%20Reference) (OtherActor :type Actor%20Object%20Reference) (OtherComp :type Primitive%20Component%20Object%20Reference) (OtherBodyIndex :type Integer))
  ;[1 0 0.7416] Makes overlapped actor invalid
  (Variables|Default|SetOverlappedActor 0))

(event Custom|Retract
  ;[1 0 0.7416] Makes the spikes appear once the event "activate trap" is called (inherited from BP_TrapBase)
  (bind _newtrack_0 (Timeline|Move ReverseFromEnd)
    (:Update
      (Transformation|SetRelativeLocation (Variables|Default|GetCone) (Math|Vector|Lerp(Vector) (Variables|Default|GetStart) (Variables|Default|GetEnd) _newtrack_0) false false))
    (:Finished
      (Utilities|FlowControl|Delay 2.0)
      (Utilities|FlowControl|DoOnce false
        (:Completed
          (CallFunction|Retract))))))

(event Custom|Redamage
  (bind _overlappedactor (Variables|Default|GetOverlappedActor))
  ;[1 0 0.7416] Applies damage to player when overlapping.
  (if (and (Utilities|IsValid _overlappedactor) (== _overlappedactor "/Game/SynthvaniaContent/Blueprints/SideScrollerCharacter.SideScrollerCharacter"))
    (Game|Damage|ApplyDamage (Variables|Default|GetOverlappedActor) 5.0 0 0)
    (Utilities|FlowControl|Delay 0.5)
    (CallFunction|Redamage)))

(event EventActivateTrap
  ;[1 0 0.7416] Makes the spikes appear once the event "activate trap" is called (inherited from BP_TrapBase)
  (Utilities|FlowControl|DoOnce false
    (:Completed
      (bind _newtrack_0 (Timeline|Move Play)
        (:Update
          (Transformation|SetRelativeLocation (Variables|Default|GetCone) (Math|Vector|Lerp(Vector) (Variables|Default|GetStart) (Variables|Default|GetEnd) _newtrack_0) false false))
        (:Finished
          (Utilities|FlowControl|Delay 2.0)
          (Utilities|FlowControl|DoOnce false
            (:Completed
              (CallFunction|Retract))))))))

(fn ConstructionScript
  (|CallParentFunction))