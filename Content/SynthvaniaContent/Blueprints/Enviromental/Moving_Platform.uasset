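; Moving platform actor that travels 400 units along world X in a direction set by the OppositeDirection flag.
; On BeginPlay, the flag selects either ForwardMovement (negative X) or BackwardMovement (positive X).
; Each caches the Cube's world location, then drives a timeline that lerps the actor from it without sweep.
; When its timeline finishes, each event calls itself again from the new location, never switching to the other.
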(event Custom|Forward%20Movement
  (Variables|Default|SetPlatform%20Current%20Location (Transformation|GetWorldLocation (Variables|Default|GetCube)))
  (bind _newtrack_0 (Timeline|Movement PlayFromStart)
    (:Update
      (Transformation|SetActorLocation (Math|Vector|Lerp(Vector) (Variables|Default|GetPlatform%20Current%20Location) (+ (Variables|Default|GetPlatform%20Current%20Location) "-400.000000,0.000000, 0") _newtrack_0) false false))
    (:Finished
      (CallFunction|ForwardMovement))))

(event Custom|Movement%20Check
  (if (Variables|Default|GetOpposite%20Direction)
    (CallFunction|BackwardMovement)
    (else
      (CallFunction|ForwardMovement))))

(event Custom|Backward%20Movement
  (Variables|Default|SetPlatform%20Current%20Location (Transformation|GetWorldLocation (Variables|Default|GetCube)))
  (bind _newtrack_0 (Timeline|Timeline_0 PlayFromStart)
    (:Update
      (Transformation|SetActorLocation (Math|Vector|Lerp(Vector) (Variables|Default|GetPlatform%20Current%20Location) (+ (Variables|Default|GetPlatform%20Current%20Location) "400.000000,0.000000, 0") _newtrack_0) false false))
    (:Finished
      (CallFunction|BackwardMovement))))

(event EventBeginPlay
  (CallFunction|MovementCHeck))

(event Collision|EventActorBeginOverlap
  (params (OtherActor :type Actor%20Object%20Reference)))

(event EventTick
  (params (DeltaSeconds :type Float%20%28single-precision%29)))

(fn ConstructionScript)