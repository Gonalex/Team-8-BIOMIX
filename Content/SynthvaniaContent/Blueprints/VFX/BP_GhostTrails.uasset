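; BP_GhostTrails is a short-lived afterimage actor that shows a frozen copy of the player's pose and fades it out.
; On BeginPlay it gets the SideScrollerCharacter, swaps each GhostMesh material for a dynamic MI_GhostTrails instance and copies the pose from the player's mesh.
; An Opacity timeline drives the Opacity parameter on those instances, then destroys the actor when finished.
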(event Custom|GhostTrails
  ;[0 0 1] Ghost Trails
  (for _array_element (Rendering|Material|GetMaterials (Variables|Default|GetGhostMesh))
    (bind _returnvalue (Rendering|Material|CreateDynamicMaterialInstance "/Game/SynthvaniaContent/ART/VFX/Materials/MI_GhostTrails.MI_GhostTrails" "None" :!class /Script/Engine.KismetMaterialLibrary))
    (bind _returnvalue_2 (Utilities|Array|Add (Variables|Default|GetDynamicMats) _returnvalue))
    (Rendering|Material|SetMaterial (Variables|Default|GetGhostMesh) _returnvalue_2 _returnvalue)
    (Class|PoseableMeshComponent|CopyPosefromSkeletalComponent (Variables|Default|GetGhostMesh) (Variables|/Script/Engine.Character|GetMesh (Variables|Default|GetPlayerCharacterRef)))
    (Components|Timeline|PlayfromStart (Variables|Colors|GetOpacity))))

(event EventBeginPlay
  ;[0 0 1] Ghost Trails
  (bind _asside_scroller_character (Utilities|Casting|CastToSideScrollerCharacter (Game|Player|GetPlayerPawn 0)))
  (Variables|Default|SetPlayerCharacterRef _asside_scroller_character)
  (CallFunction|GhostTrails))

(fn ConstructionScript)