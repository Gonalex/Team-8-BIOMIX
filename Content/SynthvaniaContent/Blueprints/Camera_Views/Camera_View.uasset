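; Camera trigger actor that switches the player's view when the side-scroller character enters its Hit volume, apparently for the Death encounter.
; On the first overlap only, it blends player 0's view target to its Camera and calls Phase1Idle on Death.
; The end overlap event is empty, and the logic to blend back to the character is disconnected, so this actor never restores the view.
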(event OnComponentBeginOverlap(Hit)
  (params (OverlappedComponent :type Primitive%20Component%20Object%20Reference) (OtherActor :type Actor%20Object%20Reference) (OtherComp :type Primitive%20Component%20Object%20Reference) (OtherBodyIndex :type Integer) (bFromSweep :type Boolean) (SweepResult :type Hit%20Result%20Structure%20%28by%20ref%29))
  (Utilities|Casting|CastToSideScrollerCharacter OtherActor)
  (Utilities|FlowControl|DoOnce false
    (:Completed
      (Game|Player|SetViewTargetwithBlend (Game|GetPlayerController 0) (Variables|Default|GetCamera) 2.0 "VTBlend_Linear" 0.0 false)
      (Default|Phase1Idle (Variables|Default|GetDeath)))))

(event OnComponentEndOverlap(Hit)
  (params (OverlappedComponent :type Primitive%20Component%20Object%20Reference) (OtherActor :type Actor%20Object%20Reference) (OtherComp :type Primitive%20Component%20Object%20Reference) (OtherBodyIndex :type Integer)))

(event Collision|EventActorBeginOverlap
  (params (OtherActor :type Actor%20Object%20Reference)))

(event EventTick
  (params (DeltaSeconds :type Float%20%28single-precision%29)))

(fn ConstructionScript)