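; BP_Enemy1 is an enemy that takes damage and reacts to the player's current element.
; BeginPlay caches the player and puts a health widget on its widget component.
; AnyDamage subtracts health, then Fire starts a non-stacking, three-tick burn timer, while Shock waits briefly, calls the player's ShockEnemies and turns the sphere purple.
; CheckHealth updates the widget or destroys the actor, deferred to the first tick or delay for elemental hits.
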(event Custom|FireDamage
  ;[1 0 0.7416] Enemy Damaging
  ;;[1 0 0.7416] Handles elemental damage and health checks.
  (Variables|Default|SetHealth (- (Variables|Default|GetHealth) 1.0))
  (CallFunction|CheckHealth)
  (bind _result (Math|Integer|IncrementInt (Variables|Default|GetFireCounter))
    (:%20%20
      (if (== _result 3)
        (Utilities|Time|ClearandInvalidateTimerbyHandle (Variables|Default|GetFireTimer))
        (Variables|Default|SetFireCounter 0)
        (Variables|Default|SetAlreadyLit false)))))

(event Game|Damage|EventAnyDamage
  (params (Damage :type Float%20%28single-precision%29) (DamageType :type Damage%20Type%20Object%20Reference) (InstigatedBy :type Controller%20Object%20Reference) (DamageCauser :type Actor%20Object%20Reference))
  ;[1 0 0.7416] Enemy Damaging
  ;;[1 0 0.7416] Initial damage - deals player's base damage
  (Variables|Default|SetHealth (- (Variables|Default|GetHealth) Damage))
  ;;[1 0 0.7416] Handles elemental damage and health checks.
  (switch Utilities|FlowControl|Switch|SwitchonEnum_Elements (Variables|/Game/SynthvaniaContent/Blueprints/SideScrollerCharacter.SideScrollerCharacter_C|GetCurrentElement (Variables|Default|GetPlayerRef))
    (:NewEnumerator0
      (if (not (Variables|Default|GetAlreadyLit))
        (Variables|Default|SetAlreadyLit true)
        (bind _returnvalue (Utilities|Time|SetTimerbyEvent (delegate Custom|FireDamage) 1.0 true))
        (Variables|Default|SetFireTimer _returnvalue)))
    (:NewEnumerator1
      (Utilities|FlowControl|Delay 0.5)
      (Default|ShockEnemies (Variables|Default|GetPlayerRef) self (Transformation|GetActorLocation))
      (Rendering|Material|SetMaterial (Variables|Default|GetSphere) 0 "/Game/SynthvaniaContent/ART/TEMP/Materials/MI_Purple.MI_Purple")
      (Utilities|FlowControl|Delay 0.2)
      (CallFunction|CheckHealth))
    (:NewEnumerator3
      (CallFunction|CheckHealth))))

(event EventBeginPlay
  ;[1 0 0.7416] Player ref for organisation.
  (bind _asside_scroller_character (Utilities|Casting|CastToSideScrollerCharacter (Game|Player|GetPlayerPawn 0)))
  (Variables|Default|SetPlayerRef _asside_scroller_character)
  (bind _returnvalue (UserInterface|CreateWidget "/Game/SynthvaniaContent/Blueprints/Widgets/WBP_EnemyHealth.WBP_EnemyHealth_C"))
  (bind _output_get (Variables|Default|SetEnemyHealth _returnvalue))
  (UserInterface|SetWidget (Variables|Default|GetWidget) _output_get))

(fn ConstructionScript
  (|CallParentFunction))

(fn CheckHealth
  (bind _health (Variables|Default|GetHealth))
  ;[1 0 0.7416] Checks health of enemy
  (if (<= _health 0.0)
    (Actor|DestroyActor)
    (else
      (Default|Update (Variables|Default|GetEnemyHealth) _health))))