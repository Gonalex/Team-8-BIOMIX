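; BP_NeonDoorTest is a test interactive door that slides or swings open when its Open event fires.
; On BeginPlay it stores the relative transform of a PhantomDoor component as the target, so the open pose is set by placing that component.
; Open plays the OpenDoor timeline, whose Alpha blends Door from its current relative transform toward that target each update, rather than from a fixed start pose.
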(event Custom|Open
  ;[1 0 0.7416] Opens door.
  (bind _alpha (Timeline|OpenDoor Play)
    (:Update
      (Transformation|SetRelativeTransform (Variables|Default|GetDoor) (Math|Transform|Lerp(Transform) (Transformation|GetRelativeTransform (Variables|Default|GetDoor)) (Variables|Default|GetTargetTrans) _alpha) false false))))

(event EventBeginPlay
  ;[1 0 0.7416] Sets target trans for modularity.
  (Variables|Default|SetTargetTrans (Transformation|GetRelativeTransform (Variables|Default|GetPhantomDoor))))

(fn ConstructionScript)