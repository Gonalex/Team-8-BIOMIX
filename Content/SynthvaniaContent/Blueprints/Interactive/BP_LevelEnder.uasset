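; BP_LevelEnder is a level-end trigger that shows the scoreboard when the side-scroller character overlaps its Box.
; The one-shot overlap clears the game mode's timer, disables player movement, creates the Scoreboard widget with a self-reference, and switches to UI-only input.
; ScoreboardCountUp animates the score through three chained, delay-separated Timelines: fixed base score, hard-coded time bonus, then the character's ChestBonus.
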(event OnComponentBeginOverlap(Box)
  (params (OverlappedComponent :type Primitive%20Component%20Object%20Reference) (OtherActor :type Actor%20Object%20Reference) (OtherComp :type Primitive%20Component%20Object%20Reference) (OtherBodyIndex :type Integer) (bFromSweep :type Boolean) (SweepResult :type Hit%20Result%20Structure%20%28by%20ref%29))
  ;[1 0 0.7416] Prompts end screen
  (Utilities|Casting|CastToSideScrollerCharacter OtherActor)
  (Utilities|FlowControl|DoOnce false
    (:Completed
      (Utilities|Time|ClearandInvalidateTimerbyHandle (Variables|/Game/SynthvaniaContent/Blueprints/SideScrollerGameMode.SideScrollerGameMode_C|GetTimerRef (.AsSide%20Scroller%20Game%20Mode (Utilities|Casting|CastToSideScrollerGameMode (Game|GetGameMode)))))
      (Game|SetGamePaused false)
      (Pawn|Components|CharacterMovement|DisableMovement (Variables|/Script/Engine.Character|GetCharacterMovement (Game|GetPlayerCharacter 0)))
      (bind _returnvalue (UserInterface|CreateWidget "/Game/SynthvaniaContent/Blueprints/Widgets/Scoreboard/Scoreboard.Scoreboard_C" (Game|GetPlayerController 0)))
      (Variables|Default|SetScoreboard%20Ref _returnvalue)
      (Variables|/Game/SynthvaniaContent/Blueprints/Widgets/Scoreboard/Scoreboard.Scoreboard_C|SetBP_LevelEnder _returnvalue self)
      (UserInterface|Viewport|AddtoViewport _returnvalue 0)
      (Input|SetInputModeUIOnly (Game|GetPlayerController 0) _returnvalue "DoNotLock")
      (Variables|/Script/Engine.PlayerController|SetbShowMouseCursor (Game|GetPlayerController 0) true))))

(event Custom|Scoreboard%20Count%20Up
  (Utilities|FlowControl|DoOnce false
    (:Completed
      (bind _newtrack_0 (Timeline|Basic%20COunter Play)
        (:Update
          (bind _output_get (Variables|/Game/SynthvaniaContent/Blueprints/Widgets/Scoreboard/Scoreboard.Scoreboard_C|SetCurrent%20Score (Variables|Default|GetScoreboard%20Ref) (Math|Float|Truncate (Math|Float|Lerp (Math|Conversions|ToFloat(Integer) (Variables|/Game/SynthvaniaContent/Blueprints/Widgets/Scoreboard/Scoreboard.Scoreboard_C|GetCurrent%20Score (Variables|Default|GetScoreboard%20Ref))) (Math|Conversions|ToFloat(Integer) (+ 0 5000)) _newtrack_0)))))
        (:Finished
          (Variables|Default|SetScore%20Reserve (Variables|/Game/SynthvaniaContent/Blueprints/Widgets/Scoreboard/Scoreboard.Scoreboard_C|GetCurrent%20Score (Variables|Default|GetScoreboard%20Ref)))
          (Utilities|Casting|CastToSideScrollerGameMode (Game|GetGameMode))
          (Variables|Default|SetTimeBonus 1234)
          (Utilities|FlowControl|Delay 1.5)
          (bind _newtrack_0_2 (Timeline|Timeline_0 Play)
            (:Update
              (Variables|/Game/SynthvaniaContent/Blueprints/Widgets/Scoreboard/Scoreboard.Scoreboard_C|SetCurrent%20Score (Variables|Default|GetScoreboard%20Ref) (Math|Float|Truncate (Math|Float|Lerp (Math|Conversions|ToFloat(Integer) _output_get) (Math|Conversions|ToFloat(Integer) (+ (Variables|Default|GetScore%20Reserve) (Variables|Default|GetTimeBonus))) _newtrack_0_2))))
            (:Finished
              (Variables|Default|SetScore%20Reserve (Variables|/Game/SynthvaniaContent/Blueprints/Widgets/Scoreboard/Scoreboard.Scoreboard_C|GetCurrent%20Score (Variables|Default|GetScoreboard%20Ref)))
              (Utilities|FlowControl|Delay 1.5)
              (bind _asside_scroller_character (Utilities|Casting|CastToSideScrollerCharacter (Game|GetPlayerCharacter 0)))
              (bind _newtrack_0_3 (Timeline|Timeline_1 Play)
                (:Update
                  (Variables|/Game/SynthvaniaContent/Blueprints/Widgets/Scoreboard/Scoreboard.Scoreboard_C|SetCurrent%20Score (Variables|Default|GetScoreboard%20Ref) (Math|Float|Truncate (Math|Float|Lerp (Math|Conversions|ToFloat(Integer) (Variables|Default|GetScore%20Reserve)) (Math|Conversions|ToFloat(Integer) (+ (Variables|Default|GetScore%20Reserve) (Variables|/Game/SynthvaniaContent/Blueprints/SideScrollerCharacter.SideScrollerCharacter_C|GetChestBonus _asside_scroller_character))) _newtrack_0_3))))))))))))

(fn ConstructionScript)