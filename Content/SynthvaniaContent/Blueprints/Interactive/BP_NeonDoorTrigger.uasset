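; Pressure plate trigger that opens a linked door when the SideScrollerCharacter steps on it.
; The box overlap plays the MoveButton timeline, which lerps the plate mesh's relative scale between Start and End vectors.
; When the timeline finishes, OpenDoor calls Open on the Door actor reference, which is assigned per instance in the level.
; No end-overlap logic resets the plate or closes the door.
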(event OnComponentBeginOverlap(Box)
  (params (OverlappedComponent :type Primitive%20Component%20Object%20Reference) (OtherActor :type Actor%20Object%20Reference) (OtherComp :type Primitive%20Component%20Object%20Reference) (OtherBodyIndex :type Integer) (bFromSweep :type Boolean) (SweepResult :type Hit%20Result%20Structure%20%28by%20ref%29))
  ;[1 0 0.7416] When player walks over plate, the door set in the public variable opens - needs to be set in viewport.
  (Utilities|Casting|CastToSideScrollerCharacter OtherActor)
  (bind _alpha (Timeline|MoveButton Play)
    (:Update
      (Transformation|SetRelativeScale3D (Variables|Default|GetSM_Box) (Math|Vector|Lerp(Vector) (Variables|Default|GetStart) (Variables|Default|GetEnd) _alpha)))
    (:Finished
      (CallFunction|OpenDoor))))

(event Custom|OpenDoor
  ;[1 0 0.7416] Calls function in the door actor
  (Default|Open (Variables|Default|GetDoor)))

(fn ConstructionScript)