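; Interactive loot chest that gives the side-scroller player a random short or large sword with a random element.
; Box overlap enables input and opens a gate, so Interact works only while the player is near.
; The first press swings the mesh open on a timeline, then rolls the weapon and displays it tinted by element.
; A later press equips it and removes the display and trigger; an older randomisation chain is left unconnected.
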(event OnComponentBeginOverlap(Box)
  (params (OverlappedComponent :type Primitive%20Component%20Object%20Reference) (OtherActor :type Actor%20Object%20Reference) (OtherComp :type Primitive%20Component%20Object%20Reference) (OtherBodyIndex :type Integer) (bFromSweep :type Boolean) (SweepResult :type Hit%20Result%20Structure%20%28by%20ref%29))
  ;[1 0 0.7416] When player interacts with chest, sets a new random weapon and new random element and then calls update function (Needs to open chest using timeline).
  (Utilities|Casting|CastToSideScrollerCharacter OtherActor)
  (Input|EnableInput (Game|GetPlayerController 0))
  (Utilities|FlowControl|Gate true) ; enters at Open
)

(event OnComponentEndOverlap(Box)
  (params (OverlappedComponent :type Primitive%20Component%20Object%20Reference) (OtherActor :type Actor%20Object%20Reference) (OtherComp :type Primitive%20Component%20Object%20Reference) (OtherBodyIndex :type Integer))
  ;[1 0 0.7416] When player interacts with chest, sets a new random weapon and new random element and then calls update function (Needs to open chest using timeline).
  (Utilities|Casting|CastToSideScrollerCharacter OtherActor)
  (Input|DisableInput (Game|GetPlayerController 0))
  (Utilities|FlowControl|Gate true) ; enters at Close
)

(event Custom|Randomise
  ;[1 0 0.7416] When player interacts with chest, sets a new random weapon and new random element and then calls update function (Needs to open chest using timeline).
  (bind (_weaponstats _element) (CallFunction|RandomWeapon))
  (Components|StaticMesh|SetStaticMesh (Variables|Default|GetWeapon) (.mesh _weaponstats))
  (switch Utilities|FlowControl|Switch|SwitchonEnum_Elements _element
    (:NewEnumerator0
      (Variables|Default|SetElementalColour "/Game/SynthvaniaContent/ART/Materials/MI_Red.MI_Red"))
    (:NewEnumerator1
      (Variables|Default|SetElementalColour "/Game/SynthvaniaContent/ART/Materials/MI_Purple.MI_Purple"))
    (:NewEnumerator2
      (Variables|Default|SetElementalColour "/Game/SynthvaniaContent/ART/Materials/MI_Blue.MI_Blue"))
    (:NewEnumerator3
      (Variables|Default|SetElementalColour 0)))
  (Rendering|Material|SetMaterial (Variables|Default|GetWeapon) 0 (Variables|Default|GetElementalColour)))

(event EventBeginPlay
  ;[1 0 0.7416] Gets player ref for organisation.
  (bind _asside_scroller_character (Utilities|Casting|CastToSideScrollerCharacter (Game|Player|GetPlayerPawn 0)))
  (Variables|Default|SetPlayerRef _asside_scroller_character))

(event Input|ActionEvents|InputActionInteract
  (params (Key :type Key%20Structure))
  ;[1 0 0.7416] When player interacts with chest, sets a new random weapon and new random element and then calls update function (Needs to open chest using timeline).
  (:Pressed
    (Utilities|FlowControl|Gate true
      (:Exit
        (if (Variables|Default|GetIsOpen)
          (Variables|/Game/SynthvaniaContent/Blueprints/SideScrollerCharacter.SideScrollerCharacter_C|SetCurrentWeapon (Variables|Default|GetPlayerRef) (Variables|Default|GetWeaponStruct))
          (Default|UpdateWeapon (Variables|Default|GetPlayerRef) (Variables|Default|GetItemElement))
          (Components|DestroyComponent (Variables|Default|GetWeapon))
          (Components|DestroyComponent (Variables|Default|GetBox))
          (else
            (bind _alpha (Timeline|OpenChest Play)
              (:Update
                (Transformation|SetRelativeRotation (Variables|Default|GetStaticMesh) (Math|Rotator|Lerp(Rotator) (Variables|Default|GetStart) (Variables|Default|GetEnd) _alpha) false false))
              (:Finished
                (Variables|Default|SetIsOpen true)
                (CallFunction|Randomise)))))))))

(fn ConstructionScript)

(fn RandomWeapon
  ;[1 0 0.7416] Randomises weapon.
  (switch int (Math|Random|RandomIntegerinRange 0 1)
    (:0
      (Variables|Default|SetWeaponStruct (Variables|/Game/SynthvaniaContent/Blueprints/SideScrollerCharacter.SideScrollerCharacter_C|GetShortSword (Variables|Default|GetPlayerRef))))
    (:1
      (Variables|Default|SetWeaponStruct (Variables|/Game/SynthvaniaContent/Blueprints/SideScrollerCharacter.SideScrollerCharacter_C|GetLargeSword (Variables|Default|GetPlayerRef)))))
  (switch int (Math|Random|RandomIntegerinRange 0 3)
    (:0
      (bind _output_get (Variables|Default|SetItemElement "NewEnumerator0"))
      (return (Variables|Default|GetWeaponStruct) _output_get))
    (:1
      (bind _output_get_2 (Variables|Default|SetItemElement "NewEnumerator1"))
      (return (Variables|Default|GetWeaponStruct) _output_get_2))
    (:2
      (bind _output_get_3 (Variables|Default|SetItemElement "NewEnumerator2"))
      (return (Variables|Default|GetWeaponStruct) _output_get_3))
    (:3
      (bind _output_get_4 (Variables|Default|SetItemElement "NewEnumerator3"))
      (return (Variables|Default|GetWeaponStruct) _output_get_4))))