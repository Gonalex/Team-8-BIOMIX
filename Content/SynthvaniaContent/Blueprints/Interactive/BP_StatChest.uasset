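; BP_StatChest is an interactable chest that opens on a key press and rolls a random stat increase.
; Box overlap with the player character enables input and opens a gate for the Interact action.
; The first press plays a timeline that rotates the mesh open; presses after it finishes call UpdateStatsElements, which only sets StatIncrease to one of three values.
; Older weapon and element randomisation logic remains in the graph, disconnected.
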(event OnComponentBeginOverlap(Box)
  (params (OverlappedComponent :type Primitive%20Component%20Object%20Reference) (OtherActor :type Actor%20Object%20Reference) (OtherComp :type Primitive%20Component%20Object%20Reference) (OtherBodyIndex :type Integer) (bFromSweep :type Boolean) (SweepResult :type Hit%20Result%20Structure%20%28by%20ref%29))
  ;[1 0 0.7416] When player interacts with chest, sets a new random weapon and new random element and then calls update function (Needs to open chest using timeline).
  (Utilities|Casting|CastToSideScrollerCharacter OtherActor)
  (Input|EnableInput (Game|GetPlayerController 0))
  (Utilities|FlowControl|Gate true) ; enters at Open
)

(event OnComponentEndOverlap(Box)
  (params (OverlappedComponent :type Primitive%20Component%20Object%20Reference) (OtherActor :type Actor%20Object%20Reference) (OtherComp :type Primitive%20Component%20Object%20Reference) (OtherBodyIndex :type Integer))
  ;[1 0 0.7416] When player interacts with chest, sets a new random weapon and new random element and then calls update function (Needs to open chest using timeline).
  (Utilities|Casting|CastToSideScrollerCharacter OtherActor)
  (Input|DisableInput (Game|GetPlayerController 0))
  (Utilities|FlowControl|Gate true) ; enters at Close
)

(event EventBeginPlay
  ;[1 0 0.7416] Gets player ref for organisation.
  (bind _asside_scroller_character (Utilities|Casting|CastToSideScrollerCharacter (Game|Player|GetPlayerPawn 0)))
  (Variables|Default|SetPlayerRef _asside_scroller_character))

(event Input|ActionEvents|InputActionInteract
  (params (Key :type Key%20Structure))
  ;[1 0 0.7416] When player interacts with chest, sets a new random weapon and new random element and then calls update function (Needs to open chest using timeline).
  (:Pressed
    (Utilities|FlowControl|Gate true
      (:Exit
        (if (Variables|Default|GetIsOpen)
          (CallFunction|UpdateStats/Elements)
          (else
            (bind _alpha (Timeline|OpenChest Play)
              (:Update
                (Transformation|SetRelativeRotation (Variables|Default|GetStaticMesh) (Math|Rotator|Lerp(Rotator) (Variables|Default|GetStart) (Variables|Default|GetEnd) _alpha) false false))
              (:Finished
                (Variables|Default|SetIsOpen true)))))))))

(fn ConstructionScript)

(fn UpdateStats/Elements
  ;[1 0 0.7416] Randomises weapon.
  (switch int (Math|Random|RandomIntegerinRange 0 2)
    (:0
      (Variables|Default|SetStatIncrease 0.5))
    (:1
      (Variables|Default|SetStatIncrease 0.75))
    (:2
      (Variables|Default|SetStatIncrease 1.0))))