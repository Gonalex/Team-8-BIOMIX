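; Spline mesh builder actor that generates surface mesh pieces along its SplineLine component in the editor.
; The construction script adds one spline mesh component per segment, assigns SurfaceMesh and SurfaceMaterial, and attaches it to the root.
; Start and end positions and tangents are both read in local space at the same point index, with no next-point offset.
; The event graph holds only disabled placeholder events.
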(event EventBeginPlay)

(event Collision|EventActorBeginOverlap
  (params (OtherActor :type Actor%20Object%20Reference)))

(event EventTick
  (params (DeltaSeconds :type Float%20%28single-precision%29)))

(fn ConstructionScript
  ;[0 1 0.083] Spline System
  (for _index (range 0 (- (Spline|GetNumberOfSplinePoints (Variables|Default|GetSpline_Line)) 2))
    (bind _returnvalue (AddComponent|AddSplineMeshComponent false (Variables|Default|GetTransform)))
    (Components|StaticMesh|SetStaticMesh _returnvalue (Variables|Default|GetSurface%20Mesh))
    (Rendering|Material|SetMaterial _returnvalue 0 (Variables|Default|GetSurface%20Material))
    (Transformation|AttachComponentToComponent _returnvalue (Variables|Default|GetDefaultSceneRoot) "None" "KeepRelative" "KeepRelative" "KeepRelative" true)
    (SplineMesh|SetStartandEnd _returnvalue (.Location (Spline|GetLocationandTangentatSplinePoint (Variables|Default|GetSpline_Line) _index "Local")) (.Tangent (Spline|GetLocationandTangentatSplinePoint (Variables|Default|GetSpline_Line) _index "Local")) (.Location (Spline|GetLocationandTangentatSplinePoint (Variables|Default|GetSpline_Line) _index "Local")) (.Tangent (Spline|GetLocationandTangentatSplinePoint (Variables|Default|GetSpline_Line) _index "Local")) true :!class /Script/Engine.SplineMeshComponent)))